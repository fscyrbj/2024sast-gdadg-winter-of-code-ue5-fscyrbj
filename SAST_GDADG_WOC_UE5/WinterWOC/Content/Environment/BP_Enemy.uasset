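; BP_Enemy is a shootable-style enemy actor that awards the player a point when killed and then respawns.
; TakeDamage prints a fixed damage label and subtracts the incoming Damage from EnemyHealth.
; At zero health or below it saves its location, destroys itself, increments the BP_FirstPersonCharacter score, then spawns a fresh BP_Enemy at that location.
; The respawn only runs if the player cast succeeds; Tick and the construction script are empty.
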(event EventTick
  (params (DeltaSeconds :type Float%20%28single-precision%29)))

(fn ConstructionScript)

(fn TakeDamage
  (params (Damage :type Integer))
  (Development|PrintText "-40")
  (bind _output_get (Variables|Default|SetEnemyHealth (- (Variables|Default|GetEnemyHealth) Damage)))
  (if (<= _output_get 0)
    (bind _output_get_2 (Variables|Default|Set位置 (Transformation|GetActorLocation)))
    (Actor|DestroyActor)
    (bind _asbp_first_person_character (Utilities|Casting|CastToBP_FirstPersonCharacter (Game|Player|GetPlayerPawn 0)))
    (Default|分数加一 _asbp_first_person_character)
    (Game|SpawnActorfromClass "BP_Enemy_C" (Math|Conversions|ToTransform(Vector) _output_get_2) "Undefined" "MultiplyWithRoot" 0 0)))